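; A speed boost pickup actor that speeds up a character that touches it.
; On overlap with a CharacterBP it sets that character's SpeedScale to 1.5, then destroys itself.
; Tick also destroys it once its game time since creation reaches five seconds.
; Both paths go through ServerDestroyself, which only destroys the actor when it has network authority.
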(event Custom|ServerDestroyself
  (Networking|SwitchHasAuthority
    (:Authority
      (Actor|DestroyActor))))

(event EventBeginPlay)

(event EventTick
  (params (DeltaSeconds :type Float%20%28single-precision%29))
  (if (>= (Actor|GetGameTimeSinceCreation) 5.0)
    (CallFunction|ServerDestroyself)))

(event Collision|EventActorBeginOverlap
  (params (OtherActor :type Actor%20Object%20Reference))
  (bind _ascharacter_bp (Utilities|Casting|CastToCharacterBP OtherActor))
  (Variables|/Game/Character/CharacterBP.CharacterBP_C|SetSpeedScale _ascharacter_bp 1.5)
  (CallFunction|ServerDestroyself))

(fn ConstructionScript)