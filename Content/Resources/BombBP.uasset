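; Bomberman-style bomb actor that explodes about four seconds after spawning and can be kicked along with an impulse.
; Two boxes (BoxX, BoxY) form the cross blast, resetting players and destroying blocks and strongholds on the server, adjusting the owning character's score.
; Destroyed blocks randomly drop speed or range pickups.
; While idle it spawns owned translucent tiles over floor tiles in range, removed when it explodes.
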(event Custom|BombExplode
  ;[1 1 1] ExplosionEvent
  (Networking|SwitchHasAuthority
    (:Authority
      (Game|SpawnActorfromClass "/Game/ExplosionBP.ExplosionBP_C" (Transformation|GetActorTransform) "Undefined" 0 0)
      (CallFunction|DestroyBombRangeTIle)
      (Actor|DestroyActor)
      (CallFunction|PlaySound))))

(event Custom|DestroyBlockEvent
  ;[1 1 1] ExplosionEvent
  (Networking|SwitchHasAuthority
    (:Authority
      (CallFunction|DestroySurroundBlocks))))

(event Custom|ServerSpawnBombRangeTile
  ;[1 1 1] ExplosionEvent
  (Networking|SwitchHasAuthority
    (:Authority
      (CallFunction|SpawnBombRangeTile))))

(event Custom|DestroyPlayer
  ;[1 1 1] ExplosionEvent
  (Networking|SwitchHasAuthority
    (:Authority
      (CallFunction|DestroySurroundPlayer))))

(event Custom|DestroyStrongholdEvent
  ;[1 1 1] ExplosionEvent
  (Networking|SwitchHasAuthority
    (:Authority
      (CallFunction|DestroySurroundStrongholds))))

(event Custom|BombMoveEvent
  (params (Moving%20direction :type Vector))
  ;[1 1 1] BombKicked
  (CallFunction|BombMoving Moving%20direction))

(event Custom|PlaySound
  ;[1 1 1] ExplosionEvent
  (CallFunction|PlayBombDestroySound))

(event EventBeginPlay
  ;[1 1 1] ExplosionEvent
  (Variables|Default|Settimer 0.0))

(event EventTick
  (params (DeltaSeconds :type Float%20%28single-precision%29))
  ;[1 1 1] ExplosionEvent
  (CallFunction|ServerSpawnBombRangeTile)
  (bind _output_get (Variables|Default|Settimer (Actor|GetGameTimeSinceCreation)))
  (if (> _output_get 4.0)
    (CallFunction|DestroyPlayer)
    (CallFunction|DestroyBlockEvent)
    (CallFunction|DestroyStrongholdEvent)
    (CallFunction|BombExplode)))

(fn ConstructionScript)

(fn BombMoving
  (params (MovingDirection :type Vector))
  (Physics|AddImpulse (Variables|Default|GetStaticMesh) (* MovingDirection 8e+02) "None" true))

(fn DestroySurroundBlocks
  (bind _returnvalue (Math|Random|RandomIntegerinRange 0 10))
  (bind _returnvalue_2 (Math|Random|RandomIntegerinRange 0 5))
  (for _array_element (Collision|GetOverlappingActors (Variables|Default|GetBox_X) "/Game/MapBlockBP.MapBlockBP_C" :!class /Script/Engine.PrimitiveComponent)
    (bind _asmap_block_bp (Utilities|Casting|CastToMapBlockBP _array_element))
    (if (== _returnvalue 0)
      (Game|SpawnActorfromClass "/Game/Resources/SpeedUpBP.SpeedUpBP_C" (Math|Conversions|ToTransform(Vector) (Transformation|GetActorLocation _asmap_block_bp)) "AdjustIfPossibleButAlwaysSpawn" 0 0)
      (elif (== _returnvalue 1)
        (Game|SpawnActorfromClass "/Game/Resources/RangeBP.RangeBP_C" (Math|Conversions|ToTransform(Vector) (Transformation|GetActorLocation _asmap_block_bp)) "AdjustIfPossibleButAlwaysSpawn" 0 0)))
    (Default|DestroySelf _asmap_block_bp)
    (CallFunction|AddScore))
  (for _array_element_2 (Collision|GetOverlappingActors (Variables|Default|GetBox_Y) "/Game/MapBlockBP.MapBlockBP_C" :!class /Script/Engine.PrimitiveComponent)
    (bind _asmap_block_bp_2 (Utilities|Casting|CastToMapBlockBP _array_element_2))
    (if (== _returnvalue_2 0)
      (Game|SpawnActorfromClass "/Game/Resources/SpeedUpBP.SpeedUpBP_C" (Math|Conversions|ToTransform(Vector) (Transformation|GetActorLocation _asmap_block_bp_2)) "AdjustIfPossibleButAlwaysSpawn" 0 0)
      (elif (== _returnvalue_2 1)
        (Game|SpawnActorfromClass "/Game/Resources/RangeBP.RangeBP_C" (Math|Conversions|ToTransform(Vector) (Transformation|GetActorLocation _asmap_block_bp_2)) "AdjustIfPossibleButAlwaysSpawn" 0 0)))
    (Default|DestroySelf _asmap_block_bp_2)
    (CallFunction|AddScore)))

(fn PlayBombDestroySound
  (bind _returnvalue (AddComponent|AddAudioComponent false))
  (Audio|Components|Audio|Play _returnvalue 0.0)
  (Transformation|SetWorldLocation _returnvalue (Transformation|GetActorLocation) false false))

(fn DestroySurroundPlayer
  (for _array_element (Collision|GetOverlappingActors (Variables|Default|GetBox_X) "/Game/Character/CharacterBP.CharacterBP_C" :!class /Script/Engine.PrimitiveComponent)
    (bind _ascharacter_bp (Utilities|Casting|CastToCharacterBP _array_element))
    (Default|ResetPlayer _ascharacter_bp)
    (CallFunction|MinusScore))
  (for _array_element_2 (Collision|GetOverlappingActors (Variables|Default|GetBox_Y) "/Game/Character/CharacterBP.CharacterBP_C" :!class /Script/Engine.PrimitiveComponent)
    (bind _ascharacter_bp_2 (Utilities|Casting|CastToCharacterBP _array_element_2))
    (Default|ResetPlayer _ascharacter_bp_2)
    (CallFunction|MinusScore)))

(fn AddScore
  (bind _ascharacter_bp (Utilities|Casting|CastToCharacterBP (Components|GetOwner self)))
  (bind _output_get (Variables|/Game/Character/CharacterBP.CharacterBP_C|SetScore _ascharacter_bp (+ (Variables|/Game/Character/CharacterBP.CharacterBP_C|GetScore _ascharacter_bp) 100)))
  (Development|PrintString (Utilities|String|ToString(Integer) _output_get)))

(fn MinusScore
  (bind _ascharacter_bp (Utilities|Casting|CastToCharacterBP (Components|GetOwner self)))
  (bind _output_get (Variables|/Game/Character/CharacterBP.CharacterBP_C|SetScore _ascharacter_bp (- (Variables|/Game/Character/CharacterBP.CharacterBP_C|GetScore _ascharacter_bp) 500)))
  (Development|PrintString (Utilities|String|ToString(Integer) _output_get)))

(fn SpawnBombRangeTile
  (bind _box_x (Variables|Default|GetBox_X))
  (bind _overlappingactors (Collision|GetOverlappingActors _box_x "/Game/MapFloorTileBP.MapFloorTileBP_C" :!class /Script/Engine.PrimitiveComponent))
  (if (> (Utilities|Array|Length _overlappingactors) 0)
    (if (not (Variables|Default|GetRangeTileSpawn))
      (for _array_element _overlappingactors
        (Game|SpawnActorfromClass "/Game/TransFloorBP.TransFloorBP_C" (Math|Transform|MakeTransform (+ (.Location (Math|Transform|BreakTransform (Transformation|GetActorTransform _array_element))) "0,0.000000,0.500000") "0, 0, 0" (.Scale (Math|Transform|BreakTransform (Transformation|GetActorTransform _array_element)))) "Undefined" self 0))
      (for _array_element_2 (Collision|GetOverlappingActors (Variables|Default|GetBox_Y) "/Game/MapFloorTileBP.MapFloorTileBP_C" :!class /Script/Engine.PrimitiveComponent)
        (Game|SpawnActorfromClass "/Game/TransFloorBP.TransFloorBP_C" (Math|Transform|MakeTransform (+ (.Location (Math|Transform|BreakTransform (Transformation|GetActorTransform _array_element_2))) "0,0.000000,0.500000") "0, 0, 0" (.Scale (Math|Transform|BreakTransform (Transformation|GetActorTransform _array_element_2)))) "Undefined" self 0))
      (Variables|Default|SetRangeTileSpawn true)
      (Variables|Default|SetRangeTileDestroy false))
    (elif (not (Variables|Default|GetRangeTileDestroy))
      (CallFunction|DestroyBombRangeTIle)
      (Variables|Default|SetRangeTileDestroy true)
      (Variables|Default|SetRangeTileSpawn false))))

(fn DestroyBombRangeTIle
  (bind _outactors (Actor|GetAllActorsOfClass "/Game/TransFloorBP.TransFloorBP_C"))
  (for _array_element _outactors
    (if (== (Components|GetOwner _array_element) self)
      (Actor|DestroyActor _array_element))))

(fn DestroySurroundStrongholds
  (for _array_element (Collision|GetOverlappingActors (Variables|Default|GetBox_X) "/Game/StrongholdBP.StrongholdBP_C" :!class /Script/Engine.PrimitiveComponent)
    (bind _asstronghold_bp (Utilities|Casting|CastToStrongholdBP _array_element))
    (Default|DestroyStronghold _asstronghold_bp)
    (CallFunction|AddScore))
  (for _array_element_2 (Collision|GetOverlappingActors (Variables|Default|GetBox_Y) "/Game/StrongholdBP.StrongholdBP_C" :!class /Script/Engine.PrimitiveComponent)
    (bind _asstronghold_bp_2 (Utilities|Casting|CastToStrongholdBP _array_element_2))
    (Default|DestroyStronghold _asstronghold_bp_2)
    (CallFunction|AddScore)))