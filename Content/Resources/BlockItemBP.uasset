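; BlockItemBP is a pickup actor that increases a character's block count when touched.
; An overlap with a CharacterBP calls its BlockNumUp, then calls ServerDestroySelf, which destroys the item only on authority.
; BeginPlay also requests destruction if the actor's age is at least 20 seconds, a check that runs only once at startup rather than on a timer.
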(event Custom|ServerDestroySelf
  (Networking|SwitchHasAuthority
    (:Authority
      (Actor|DestroyActor))))

(event EventBeginPlay
  (if (>= (Actor|GetGameTimeSinceCreation) 2e+01)
    (CallFunction|ServerDestroyself)))

(event Collision|EventActorBeginOverlap
  (params (OtherActor :type Actor%20Object%20Reference))
  (bind _ascharacter_bp (Utilities|Casting|CastToCharacterBP OtherActor))
  (Default|BlockNumUp _ascharacter_bp)
  (CallFunction|ServerDestroySelf))

(event EventTick
  (params (DeltaSeconds :type Float%20%28single-precision%29)))

(fn ConstructionScript)