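; Player controller that gives the local player a hold-to-view minimap.
; On BeginPlay, the local controller creates the WidgetHud widget, adds it to the viewport hidden, then shows it only while OpenMinimap input is held.
; BeginPlay also calls ToggleVisibility, which, despite its name, only makes the controlled CharacterBP's Cone component visible, and only on authority.
; An older press-to-toggle minimap branch remains disconnected.
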(event Custom|ToggleVisibility
  (Networking|SwitchHasAuthority
    (:Authority
      (bind _ascharacter_bp (Utilities|Casting|CastToCharacterBP (Pawn|GetControlledPawn self)))
      (Rendering|SetVisibility (Variables|/Game/Character/CharacterBP.CharacterBP_C|GetCone _ascharacter_bp) true false))))

(event EventBeginPlay
  (bind _self self)
  (CallFunction|ToggleVisibility)
  (if (Pawn|IsLocalPlayerController _self)
    (bind _returnvalue (UserInterface|CreateWidget "/Game/Character/Minimap/WidgetHud.WidgetHud_C" _self))
    (bind _output_get (Variables|Default|SetMinimapRef _returnvalue))
    (UserInterface|Viewport|AddtoViewport _output_get 0)
    (Widget|SetVisibility _output_get "Hidden")))

(event EventTick
  (params (DeltaSeconds :type Float%20%28single-precision%29)))

(event Input|ActionEvents|InputActionOpenMinimap
  (params (Key :type Key%20Structure))
  (bind _minimapref (Variables|Default|GetMinimapRef))
  (:Pressed
    (Widget|SetVisibility _minimapref "Visible"))
  (:Released
    (Widget|SetVisibility _minimapref "Hidden")))

(fn ConstructionScript)