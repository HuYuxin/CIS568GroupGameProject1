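; HUD Blueprint that puts the in-game UI on screen and handles the end-of-match display.
; BeginPlay creates the timer, score and resource widgets for the owning player and adds them to the viewport.
; DisplayWinLossByWinBoolean prints a debug string, shows the TimeUpWinLoss widget, then loads the MainMenu level after a short delay.
; An unconnected WidgetHud creation chain remains in the graph and never runs.
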(event Custom|DisplayWinLossByWinBoolean
  (Development|PrintString "Hello DisplayWinLossByWinBoolean")
  (bind _returnvalue (UserInterface|CreateWidget "/Game/TimeUpWinLoss.TimeUpWinLoss_C" (Variables|Default|GetPlayerOwner)))
  (UserInterface|Viewport|AddtoViewport _returnvalue 0)
  (Utilities|FlowControl|Delay 5.0)
  (Game|OpenLevel(byName) "MainMenu"))

(event EventBeginPlay
  (bind _returnvalue (UserInterface|CreateWidget "/Game/TimerWidget.TimerWidget_C" (Variables|Default|GetPlayerOwner)))
  (UserInterface|Viewport|AddtoViewport _returnvalue 0)
  (bind _returnvalue_2 (UserInterface|CreateWidget "/Game/ScoreDisplay.ScoreDisplay_C" (Variables|Default|GetPlayerOwner)))
  (UserInterface|Viewport|AddtoViewport _returnvalue_2 0)
  (bind _returnvalue_3 (UserInterface|CreateWidget "/Game/ResourceDisplay.ResourceDisplay_C" (Variables|Default|GetPlayerOwner)))
  (UserInterface|Viewport|AddtoViewport _returnvalue_3 0))

(event Collision|EventActorBeginOverlap
  (params (OtherActor :type Actor%20Object%20Reference)))

(event EventTick
  (params (DeltaSeconds :type Float%20%28single-precision%29)))

(fn ConstructionScript)