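; TransBlockBP is a destructible block that can drop a power-up at its location when it is destroyed.
; DestroySelf calls SpawnItems, then DestroyBlock, which is not defined in this Blueprint.
; SpawnItems rolls a random integer for a SpeedUpBP drop and, failing that, rolls again for a RangeBP drop, so often nothing spawns.
; The event graph and construction script hold no logic.
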(event EventBeginPlay)

(event Collision|EventActorBeginOverlap
  (params (OtherActor :type Actor%20Object%20Reference)))

(event EventTick
  (params (DeltaSeconds :type Float%20%28single-precision%29)))

(fn ConstructionScript)

(fn DestroySelf
  (CallFunction|SpawnItems)
  (Class|MapBlock|DestroyBlock))

(fn SpawnItems
  (bind _returnvalue (Math|Random|RandomIntegerinRange 0 5))
  (bind _returnvalue_2 (Transformation|GetActorLocation))
  (bind _returnvalue_3 (Math|Conversions|ToTransform(Vector) _returnvalue_2))
  (if (== _returnvalue 0)
    (Game|SpawnActorfromClass "/Game/Resources/SpeedUpBP.SpeedUpBP_C" _returnvalue_3 "AdjustIfPossibleButAlwaysSpawn" 0 0)
    (elif (== _returnvalue 1)
      (Game|SpawnActorfromClass "/Game/Resources/RangeBP.RangeBP_C" _returnvalue_3 "AdjustIfPossibleButAlwaysSpawn" 0 0))))